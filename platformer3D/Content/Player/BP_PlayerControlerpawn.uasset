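; Player controller that sets up Enhanced Input and relays player actions to the possessed BP_PlayerPawn.
; On possess, it adds the player mapping context, then casts and caches the pawn; the null-warning branch is unreachable because its condition is constant true.
; Jump, crouch, move and sprint start/stop actions call matching functions on the cached pawn, which holds the actual behavior.
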(event Input|EnhancedActionEvents|EnhancedInputActionIN_PlayerMove
  (params (ActionValue :type Vector :default "0, 0, 0") (ElapsedSeconds :type Float%20%28double-precision%29) (TriggeredSeconds :type Float%20%28double-precision%29) (InputAction :type Input%20Action%20Object%20Reference :default "/Game/Blueprint/InputSystem/PlayerInputContext/IN_PlayerMove.IN_PlayerMove"))
  (Default|MoveFunc (Variables|Default|GetplayerCharacter) ActionValue))

(event Input|EnhancedActionEvents|EnhancedInputActionIN_PlayerCrouch
  (params (ActionValue :type Boolean) (ElapsedSeconds :type Float%20%28double-precision%29) (TriggeredSeconds :type Float%20%28double-precision%29) (InputAction :type Input%20Action%20Object%20Reference :default "/Game/Blueprint/InputSystem/PlayerInputContext/IN_PlayerCrouch.IN_PlayerCrouch"))
  (Default|CrouchFunc (Variables|Default|GetplayerCharacter)))

(event Input|EnhancedActionEvents|EnhancedInputActionIN_PlayerJump
  (params (ActionValue :type Boolean) (ElapsedSeconds :type Float%20%28double-precision%29) (TriggeredSeconds :type Float%20%28double-precision%29) (InputAction :type Input%20Action%20Object%20Reference :default "/Game/Blueprint/InputSystem/PlayerInputContext/IN_PlayerJump.IN_PlayerJump"))
  (Default|JumpFunc (Variables|Default|GetplayerCharacter)))

(event Input|EnhancedActionEvents|EnhancedInputActionIN_PlayerSprint
  (params (ActionValue :type Boolean) (ElapsedSeconds :type Float%20%28double-precision%29) (TriggeredSeconds :type Float%20%28double-precision%29) (InputAction :type Input%20Action%20Object%20Reference :default "/Game/Blueprint/InputSystem/PlayerInputContext/IN_PlayerSprint.IN_PlayerSprint"))
  (bind _playercharacter (Variables|Default|GetplayerCharacter))
  (:Started
    (Default|SprintStartFunc _playercharacter))
  (:Completed
    (Default|SprintStopFunc _playercharacter)))

(event EventPossess
  (params (PossessedPawn :type Pawn%20Object%20Reference))
  (bind _returnvalue (PlayerController|LocalPlayerSubsystems|GetEnhancedInputLocalPlayerSubsystem))
  (Utilities|IsValid _returnvalue
    (:Is%20Valid
      (Input|AddMappingContext _returnvalue "/Game/Blueprint/InputSystem/MI_PlayerInputMapping.MI_PlayerInputMapping" 0 "(bIgnoreAllPressedKeysUntilRelease=True,bForceImmediately=False,bNotifyUserSettings=False)")
      (if true
        (bind _asbp_player_pawn (Utilities|Casting|CastToBP_PlayerPawn PossessedPawn))
        (Variables|Default|SetplayerCharacter _asbp_player_pawn)
        (else
          (Development|PrintString "Player character null"))))))

(fn ConstructionScript)