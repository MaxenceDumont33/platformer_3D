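; BP_PlayerPawn is a player pawn that exposes movement actions as functions, with no input handling of its own.
; MoveFunc adds movement input along the supplied direction, converted through a rotation to a forward vector.
; The sprint start and stop functions switch FloatingPawnMovement's max speed between fast and normal, printing a debug string.
; Crouch and jump are empty stubs, and Tick and the construction script do nothing.
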(event EventTick
  (params (DeltaSeconds :type Float%20%28single-precision%29)))

(fn ConstructionScript)

(fn MoveFunc
  (params (Direction :type Vector))
  (Pawn|Input|AddMovementInput (Math|Vector|GetForwardVector (Math|Conversions|RotationFromXVector Direction)) 1.0 false))

(fn CrouchFunc)

(fn JumpFunc)

(fn SprintStartFunc
  (Variables|/Script/Engine.FloatingPawnMovement|SetMaxSpeed (Variables|Default|GetFloatingPawnMovement) 1.2e+03)
  (Development|PrintString "start"))

(fn SprintStopFunc
  (Variables|/Script/Engine.FloatingPawnMovement|SetMaxSpeed (Variables|Default|GetFloatingPawnMovement) 6e+02)
  (Development|PrintString "stop"))