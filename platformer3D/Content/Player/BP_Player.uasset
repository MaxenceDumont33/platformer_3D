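; BP_Player is the player character Blueprint, built around a ParckourMovement component for parkour-style movement.
; It initializes that component on BeginPlay and forwards landing, movement mode changes and jumps to it.
; Movement input follows the camera's forward vector rotated by the input direction, and sprint start/stop switches max walk speed.
; CrouchFunc is an empty stub, and the construction script leaves the capsule visible in game.
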(event EventBeginPlay
  (Default|Initialize (Variables|Default|GetParckourMovement) self))

(event EventOnMovementModeChanged
  (params (PrevMovementMode :type EMovementMode%20Enum :default "MOVE_None") (NewMovementMode :type EMovementMode%20Enum :default "MOVE_None") (PrevCustomMode :type Byte :default 0) (NewCustomMode :type Byte :default 0))
  (Default|MovementChanged (Variables|Default|GetParckourMovement) PrevMovementMode NewMovementMode))

(event EventOnLanded
  (params (Hit :type Hit%20Result%20Structure%20%28by%20ref%29))
  (Default|LandEvent (Variables|Default|GetParckourMovement)))

(fn ConstructionScript
  (Development|SetHiddeninGame (Variables|Collision|GetCapsuleComponent) false false))

(fn MoveFunc
  (params (Direction :type Vector))
  (Pawn|Input|AddMovementInput (Math|Vector|RotateVector (Math|Vector|GetForwardVector (Variables|Default|GetCamera)) (Math|Conversions|RotationFromXVector Direction)) 1.0 false))

(fn CrouchFunc)

(fn JumpFunc
  (Character|Jump)
  (Default|Jump (Variables|Default|GetParckourMovement)))

(fn SprintStartFunc
  (Variables|/Script/Engine.CharacterMovementComponent|SetMaxWalkSpeed (Variables|Character|GetCharacterMovement) 1.2e+03))

(fn SprintStopFunc
  (Variables|/Script/Engine.CharacterMovementComponent|SetMaxWalkSpeed (Variables|Character|GetCharacterMovement) 6e+02)
  (Development|PrintString "stop"))